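; RTS gatherer unit that shuttles between a resource node and the closest same-team building, crediting the player controller on each drop-off.
; SetIsWorking picks the drop-off and starts the trip; Collect halts the unit for a timed harvest, while DropOff banks the resource and sends it back.
; Multicast events drive the particles, audio and nose material showing cargo state.
; Tick rotates the Spinner, which is registered with Body for team coloring.
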(event Custom|ResourceCollector
  (Utilities|Time|ClearandInvalidateTimerbyHandle (Variables|Default|GetResourceCollectTimer))
  (Variables|Default|SetHasResource? true)
  (CallFunction|UnitMoveCommand (Transformation|GetActorLocation (Variables|Default|GetDropOffBuilding)))
  ;[1 1 1] Multicast done collecting
  (CallFunction|MulticastDoneCollecting))

(event Custom|MulticastStartCollecting
  ;[1 1 1] Multicast start collecting
  (Components|Activation|SetActive (Variables|Default|GetParticleSystem) true false)
  (Audio|Components|Audio|Play (Variables|Default|GetAudio) 0.0))

(event Custom|MulticastDoneCollecting
  ;[1 1 1] Multicast done collecting
  (Components|Activation|SetActive (Variables|Default|GetParticleSystem) false false)
  (Audio|Components|Audio|Stop (Variables|Default|GetAudio))
  (Rendering|Material|SetMaterial (Variables|Default|GetNose) 0 "/Game/StarterContent/Materials/M_Metal_Gold.M_Metal_Gold"))

(event Custom|MulticastResourceDroppedOff
  ;[1 1 1] Multicast Resources dropped off
  (Rendering|Material|SetMaterial (Variables|Default|GetNose) 0 "/Game/StarterContent/Materials/M_Basic_Wall.M_Basic_Wall"))

(event Custom|MulticastNotWorking
  ;[1 1 1] Multicast not working
  (Components|Activation|SetActive (Variables|Default|GetParticleSystem) false false)
  (Audio|Components|Audio|Stop (Variables|Default|GetAudio)))

(event EventBeginPlay
  (|CallParentFunction) ; This node is disabled and will not be called.\nDrag off pins to build functionality.
)

(event Collision|EventActorBeginOverlap
  (params (OtherActor :type Actor%20Object%20Reference)))

(event EventTick
  (params (DeltaSeconds :type Float%20%28single-precision%29))
  (Transformation|AddRelativeRotation (Variables|Default|GetSpinner) (Math|Rotator|MakeRotator 0.0 0.0 (* DeltaSeconds 2.5e+02)) false false))

(event EventSetIsWorking
  (params (ResourceNode :type Actor%20Object%20Reference))
  (Variables|Default|SetisWorking? true)
  (Variables|Default|SetResourceNode ResourceNode)
  ;[1 1 1] Find nearest dropoff point
  (bind _outactors (Actor|GetAllActorsOfClass "/Game/RTS_Unknown/Buildings/BP_ParentBuildingClass.BP_ParentBuildingClass_C"))
  (for _array_element _outactors
    (bind _teamnumber (Default|GetTeam _array_element))
    (if (== _teamnumber (Variables|Default|GetTeamNumber))
      (if (< (Transformation|GetDistanceTo _array_element self) (Variables|Default|GetClosestDropOffBuildingDistance))
        (Variables|Default|SetDropOffBuilding _array_element)
        (Variables|Default|SetClosestDropOffBuildingDistance (Transformation|GetDistanceTo _array_element self)))))
  (if (Variables|Default|GetHasResource?)
    (CallFunction|UnitMoveCommand (Transformation|GetActorLocation (Variables|Default|GetDropOffBuilding)))
    (else
      (CallFunction|UnitMoveCommand (Transformation|GetActorLocation (Variables|Default|GetResourceNode))))))

(event EventSetNotWorking
  (Variables|Default|SetisWorking? false)
  (Utilities|Time|ClearandInvalidateTimerbyHandle (Variables|Default|GetResourceCollectTimer))
  ;[1 1 1] Multicast not working
  (CallFunction|MulticastNotWorking))

(event EventCollect
  (if (Variables|Default|GetisWorking?)
    (if (Variables|Default|GetHasResource?)
      ;[1 1 1] Already has resource, head to dropoff
      (CallFunction|UnitMoveCommand (Transformation|GetActorLocation (Variables|Default|GetDropOffBuilding)))
      (elif (not (Utilities|Time|IsValidTimerHandle (Variables|Default|GetResourceCollectTimer)))
        ;[1 1 1] Stop movement
        (CallFunction|UnitMoveCommand (Transformation|GetActorLocation))
        ;[1 1 1] Multicast start collecting
        (CallFunction|MulticastStartCollecting)
        (bind _returnvalue (Utilities|Time|SetTimerbyEvent (delegate Custom|ResourceCollector) 4.0))
        (Variables|Default|SetResourceCollectTimer _returnvalue)))))

(event EventDropOff
  (if (Variables|Default|GetisWorking?)
    ;[1 1 1] No resources, go back to resourcenode
    (if (Variables|Default|GetHasResource?)
      (Class|IResources|IncrementResourceAmount(Message) (Game|GetPlayerController (Variables|Default|GetTeamNumber)) 10)
      (Variables|Default|SetHasResource? false)
      ;[1 1 1] Multicast Resources dropped off
      (CallFunction|MulticastResourceDroppedOff)
      (CallFunction|UnitMoveCommand (Transformation|GetActorLocation (Variables|Default|GetResourceNode)))
      (else
        (CallFunction|UnitMoveCommand (Transformation|GetActorLocation (Variables|Default|GetResourceNode)))))))

(fn ConstructionScript
  (bind _meshesforteamcoloring (Variables|Default|GetMeshesForTeamColoring))
  (|CallParentFunction)
  (Utilities|Array|Add _meshesforteamcoloring (Variables|Default|GetBody))
  (Utilities|Array|Add _meshesforteamcoloring (Variables|Default|GetSpinner)))

(fn GetResourceAmount
  (return 0))