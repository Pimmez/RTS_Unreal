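; RTS player pawn that provides a spring-arm camera with smoothed zoom and rotation.
; Each tick it reads the zoom and rotate input action values and lerps stored zoom and rotation speeds toward them using delta time, giving eased start and stop.
; Zoom speed adds to the spring arm length, clamped between min and max limits, while rotation speed yaws the spring arm.
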(event EventBeginPlay)

(event Collision|EventActorBeginOverlap
  (params (OtherActor :type Actor%20Object%20Reference)))

(event EventTick
  (params (DeltaSeconds :type Float%20%28single-precision%29))
  (CallFunction|ZoomCamera)
  (CallFunction|RotateCamera))

(fn ConstructionScript)

(fn ZoomCamera
  (bind _springarm (Variables|Default|GetSpringArm))
  (bind _output_get (Variables|CameraControls|SetzoomValue (Math|Float|Lerp (Variables|CameraControls|GetzoomValue) (* (Input|EnhancedActionValues|GetIA_Zoom) 1e+02) (* (Utilities|Time|GetWorldDeltaSeconds) 5.0))))
  (Variables|/Script/Engine.SpringArmComponent|SetTargetArmLength _springarm (Math|Float|Clamp(Float) (+ (Variables|/Script/Engine.SpringArmComponent|GetTargetArmLength _springarm) _output_get) (Variables|CameraControls|GetminZoomValue) (Variables|CameraControls|GetmaxZoomValue))))

(fn RotateCamera
  (bind _output_get (Variables|CameraControls|SetrotationValue (Math|Float|Lerp (Variables|CameraControls|GetrotationValue) (* (Input|EnhancedActionValues|GetIA_RotateCamera) 1.0) (* (Utilities|Time|GetWorldDeltaSeconds) 5.0))))
  (Transformation|AddRelativeRotation (Variables|Default|GetSpringArm) (Math|Rotator|MakeRotator 0.0 0.0 _output_get) false false))