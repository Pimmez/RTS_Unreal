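; RTS game mode that gives each joining player a camera pawn, a random start camp and a team.
; The construction script gathers all BP_PlayerStartCamp actors.
; On a new player, it spawns BP_PlayerPawn at a camp's camera location, possesses it, and sends camp, team number and color via SetupPlayerStartMessage, then increments the team and removes the camp.
; GetTeam and IsOnMyTeam? return only fixed defaults.
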(event EventHandleStartingNewPlayer
  (params (NewPlayer :type Player%20Controller%20Object%20Reference))
  (bind _playerstartcamps (Variables|Default|GetPlayerStartCamps))
  (bind _outitem (Utilities|Array|Random _playerstartcamps))
  (Variables|Default|SetSelectedPlayerStartCamp _outitem)
  (Utilities|IsValid _outitem
    (:Is%20Valid
      (bind _returnvalue (Game|SpawnActorfromClass "/Game/RTS_Unknown/BP_PlayerPawn.BP_PlayerPawn_C" (Transformation|GetWorldTransform (Variables|/Game/RTS_Unknown/BP_PlayerStartCamp.BP_PlayerStartCamp_C|GetCameralocation (Variables|Default|GetSelectedPlayerStartCamp))) "Undefined" 0 0))
      (Pawn|Possess NewPlayer _returnvalue)
      (Class|IMultiplayer|SetupPlayerStart(Message) NewPlayer (Variables|Default|GetSelectedPlayerStartCamp) (Variables|Default|GetTeamNumber) (Utilities|Array|Get(acopy) (Variables|Default|GetTeamColors) (Variables|Default|GetTeamNumber)))
      (Math|Integer|IncrementInt (Variables|Default|GetTeamNumber)
        (:%20%20
          (Utilities|Array|RemoveItem (Variables|Default|GetPlayerStartCamps) (Variables|Default|GetSelectedPlayerStartCamp)))))))

(fn ConstructionScript
  (bind _outactors (Actor|GetAllActorsOfClass "/Game/RTS_Unknown/BP_PlayerStartCamp.BP_PlayerStartCamp_C"))
  (Variables|Default|SetPlayerStartCamps _outactors))

(fn GetTeam
  (return 0))

(fn IsonMyTeam?
  (params (TeamNumber :type Integer))
  (return false))