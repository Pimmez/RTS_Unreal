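; RTS player controller that handles mouse selection, unit move orders and each player's starting spawn.
; Left click selects a same-team building and drives HUD unit selection through messages.
; Right click sends the HUD's selected units to the cursor hit via ServerUnitMoveCommand and spawns a cursor effect.
; On authority, SetupPlayerStart stores team data and spawns a center building and three units at the camp's markers.
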(event Custom|ServerUnitMoveCommand
  (params (Unit :type Actor%20Object%20Reference) (Location :type Vector))
  (Class|ISelection|UnitMoveCommand(Message) Unit Location))

(event EventTick
  (params (DeltaSeconds :type Float%20%28single-precision%29))
  (if (Variables|Default|GetisLeftMousePressed?)
    (Class|ISelection|SelectionHeld(Message) (HUD|GetHUD))))

(event EventBeginPlay
  (if (Pawn|IsLocalPlayerController)
    (Input|SetInputModeGameandUI self 0 "LockAlways" false false)
    (Variables|Default|SetbShowMouseCursor true)
    (bind _returnvalue (UserInterface|CreateWidget "/Game/RTS_Unknown/Widgets/WBP_SelectedUnitArea.WBP_SelectedUnitArea_C"))
    (bind _output_get (Variables|Default|SetSelectedUnitArea _returnvalue))
    (UserInterface|Viewport|AddtoViewport _output_get 0)))

(event EventAddUnittoSelectedUnitArea
  (params (SelectedUnitWidget :type User%20Widget%20Object%20Reference))
  (Class|HorizontalBox|AddChildtoHorizontalBox (Variables|/Game/RTS_Unknown/Widgets/WBP_SelectedUnitArea.WBP_SelectedUnitArea_C|GetUnitBox (Variables|Default|GetSelectedUnitArea)) SelectedUnitWidget))

(event EventClearSelectedBuilding
  ;[1 1 1] Clear Selected Building
  (Utilities|IsValid (Variables|Default|GetSelectedBuilding)
    (:Is%20Valid
      (Class|ISelection|DeselectThis(Message) (Variables|Default|GetSelectedBuilding))
      (Variables|Default|SetSelectedBuilding 0))))

(event EventSetupPlayerStart
  (params (PlayerStartCamp :type BP%20Player%20Start%20Camp%20Object%20Reference) (TeamNumber :type Integer) (TeamColor :type Linear%20Color%20Structure))
  (Networking|SwitchHasAuthority
    (:Authority
      (Variables|Default|SetTeam%20Number TeamNumber)
      (Variables|Default|SetTeam%20Color TeamColor)
      (Utilities|InitializePlayerSpawn PlayerStartCamp))))

(event Input|MouseEvents|LeftMouseButton
  (params (Key :type Key%20Structure :default "None"))
  (bind _returnvalue (HUD|GetHUD))
  (:Pressed
    (Variables|Default|SetisLeftMousePressed? true)
    (Utilities|HandleBuildingClick)
    (Class|ISelection|SelectionPressed(Message) _returnvalue))
  (:Released
    (Variables|Default|SetisLeftMousePressed? false)
    (Class|ISelection|SelectionReleased(Message) _returnvalue)))

(event Input|MouseEvents|RightMouseButton
  (params (Key :type Key%20Structure :default "None"))
  (:Pressed
    (Variables|Default|SetrightClickLocation (.Location (Collision|BreakHitResult (.HitResult (Game|Player|GetHitResultUnderCursorbyChannel "TraceTypeQuery1" true)))))
    (bind _units (Class|ISelection|GrabSelectedUnits(Message) (HUD|GetHUD)))
    (for _array_element _units
      (CallFunction|ServerUnitMoveCommand _array_element (Variables|Default|GetrightClickLocation)))
    (Niagara|SpawnSystematLocation "/Game/LevelPrototyping/Cursor/FX_Cursor.FX_Cursor" (Variables|Default|GetrightClickLocation))))

(fn ConstructionScript)

(fn Moveto
  (params (Location :type Vector))
  (AI|Navigation|SimpleMovetoLocation self Location)
  (Niagara|SpawnSystematLocation (Variables|Input|GetFXCursor) Location))

(fn Follow
  (params (Location :type Vector))
  (bind _returnvalue (Pawn|GetControlledPawn))
  (Pawn|Input|AddMovementInput _returnvalue (Math|Vector|GetUnitDirection(Vector) (Transformation|GetActorLocation _returnvalue) Location) 1.0 false))

(fn GetLocationUnderCursor
  (bind _hitresult (Game|Player|GetHitResultUnderCursorbyChannel "TraceTypeQuery1" true))
  (bind (_bblockinghit _binitialoverlap _time _distance _location) (Collision|BreakHitResult _hitresult))
  (return _bblockinghit _location))

(fn GetLocationUnderFinger
  (bind _hitresult (Class|PlayerController|GetHitResultUnderFingerbyChannel "Touch1" "TraceTypeQuery1" false))
  (bind (_bblockinghit _binitialoverlap _time _distance _location) (Collision|BreakHitResult _hitresult))
  (return _bblockinghit _location))

(fn GetTeam
  (return 0))

(fn GrabSelectedUnits
  (return 0))

(fn IsonMyTeam?
  (params (TeamNumber :type Integer))
  (return (== TeamNumber (Variables|Default|GetTeam%20Number))))