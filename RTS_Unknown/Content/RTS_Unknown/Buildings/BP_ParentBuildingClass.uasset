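; Parent building Blueprint for an RTS, providing selection feedback and team coloring.
; On BeginPlay it creates a WBP_SelectedBuilding widget linked to itself and tints the mesh through a dynamic material's TeamColor parameter.
; Select and deselect events toggle the selection decal and add or remove that widget.
; GetTeam returns the team number, while GrabSelectedUnits and IsOnMyTeam? are stubs, the latter always returning false.
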(event EventDeselectThis
  (Rendering|SetVisibility (Variables|Default|GetSelectiveDecal) false false)
  (Widget|RemovefromParent (Variables|Default|GetBuildingSelected_Widget)))

(event EventSelectThis
  (Rendering|SetVisibility (Variables|Default|GetSelectiveDecal) true false)
  (UserInterface|Viewport|AddtoViewport (Variables|Default|GetBuildingSelected_Widget) 0))

(event EventBeginPlay
  (Utilities|FlowControl|Sequence
    (:then_0
      ;[1 1 1] Create building selected widget
      (bind _returnvalue (UserInterface|CreateWidget "/Game/RTS_Unknown/Widgets/WBP_SelectedBuilding.WBP_SelectedBuilding_C"))
      (Variables|Default|SetBuildingSelected_Widget _returnvalue)
      (Variables|/Game/RTS_Unknown/Widgets/WBP_SelectedBuilding.WBP_SelectedBuilding_C|SetBuildingReference _returnvalue self))
    (:then_1
      ;[1 1 1] Setup Teamcolor
      (bind _returnvalue_2 (Rendering|Material|CreateDynamicMaterialInstance (Rendering|Material|GetMaterial (Variables|Default|GetBuildingMesh) 0) "None" "None" :!class /Script/Engine.KismetMaterialLibrary))
      (Rendering|Material|SetVectorParameterValue _returnvalue_2 "TeamColor" (Variables|Default|GetTeamColor) :!class /Script/Engine.MaterialInstanceDynamic)
      (Rendering|Material|SetMaterial (Variables|Default|GetBuildingMesh) 0 _returnvalue_2))))

(fn ConstructionScript)

(fn GetTeam
  (return (Variables|Default|GetTeamNumber)))

(fn GrabSelectedUnits
  (return 0))

(fn IsonMyTeam?
  (params (TeamNumber :type Integer))
  (return false))